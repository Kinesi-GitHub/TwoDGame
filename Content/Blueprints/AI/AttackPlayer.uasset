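; AttackPlayer is a Behavior Tree task that lets an enemy damage the 2D side-scroller player character.
; On execute it compares the controlled pawn's distance to player 0 against Range.
; In range, it applies the BaseEnemy's Damage through the player's Health and finishes successfully; out of range, it finishes as failed.
; A failed cast of either character stops execution without calling FinishExecute.
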(event EventReceiveExecuteAI
  (params (OwnerController :type AI%20Controller%20Object%20Reference) (ControlledPawn :type Pawn%20Object%20Reference))
  (bind _returnvalue (Game|GetPlayerCharacter 0))
  (bind _as2dside_scroller_character (Utilities|Casting|CastTo2DSideScrollerCharacter _returnvalue))
  (if (<= (Transformation|GetDistanceTo ControlledPawn _returnvalue) (Variables|Default|GetRange))
    (bind _asbase_enemy (Utilities|Casting|CastToBaseEnemy ControlledPawn))
    (Default|TakeDamage (Variables|/Game/2DSideScrollerBP/Blueprints/2DSideScrollerCharacter.2DSideScrollerCharacter_C|GetHealth _as2dside_scroller_character) (Variables|/Game/Blueprints/Actors/Pawns/BaseEnemy.BaseEnemy_C|GetDamage _asbase_enemy))
    (AI|BehaviorTree|FinishExecute true)
    (else
      (AI|BehaviorTree|FinishExecute false))))