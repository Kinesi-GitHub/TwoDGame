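; Behavior Tree task that turns the AI-controlled pawn toward the Blackboard "Location" vector.
; Each execution applies one constant-speed RInterp step at RotationSpeed, then finishes successfully without waiting for alignment.
; The look-at rotation starts from the pawn's forward unit vector rather than its world position.
; It only runs while player character 0 is valid; otherwise it never calls FinishExecute.
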(event EventReceiveExecuteAI
  (params (OwnerController :type AI%20Controller%20Object%20Reference) (ControlledPawn :type Pawn%20Object%20Reference))
  (bind _returnvalue (Transformation|GetActorRotation ControlledPawn))
  (Utilities|IsValid (Game|GetPlayerCharacter 0)
    (:Is%20Valid
      (Transformation|SetActorRotation ControlledPawn (Class|KismetMathLibrary|RInterptoConstant _returnvalue (Math|Rotator|FindLookatRotation (Math|Rotator|GetRotationXVector _returnvalue) (AI|Components|Blackboard|GetValueasVector (AI|GetBlackboard OwnerController) (Utilities|Name|MakeLiteralName "Location"))) (Utilities|Time|GetWorldDeltaSeconds) (Variables|Default|GetRotationSpeed)))
      (AI|BehaviorTree|FinishExecute true))))