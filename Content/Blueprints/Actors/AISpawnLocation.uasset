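; AISpawnLocation is a one-shot spawn point that announces and then spawns a RedSqaure actor.
; On BeginPlay it plays a spawn sound and attaches a fire emitter, waits a short random delay, spawns the actor at its location, then destroys itself.
; An unconnected SpawnAIFromClass branch, using an AI pawn and BT_Basic behavior tree, never runs.
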(event EventBeginPlay
  (Audio|PlaySoundatLocation "/Game/Sounds/EnemySpawn2_Cue.EnemySpawn2_Cue" (Transformation|GetActorLocation) "0, 0, 0" 1.0 1.0 0.0 0 0 0)
  (Effects|SpawnEmitterAttached "/Game/StarterContent/Particles/P_Fire.P_Fire" (Variables|Default|GetScene) "None")
  (Utilities|FlowControl|Delay (Math|Random|RandomFloatinRange 2.0 5.0))
  (Game|SpawnActorfromClass "/Game/Blueprints/Actors/Pawns/RedSqaure.RedSqaure_C" (Math|Conversions|ToTransform(Vector) (Transformation|GetActorLocation)) "AdjustIfPossibleButAlwaysSpawn" 0 0)
  (Actor|DestroyActor))

(fn ConstructionScript)