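; Game mode for the box launch game that scatters spawnable objects across the level at start and tracks game over.
; On BeginPlay it runs SpawnObjects, plays the music and starts a looping timer for SetGameStage, which has no graph here.
; SpawnObjects places a set count of each item class at random points on the upper XZ plane, skipping blocked spots.
; OnGameOver sets a flag and casts to PlayerHUD without using it.
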(event Custom|OnGameOver
  (Variables|Default|SetGameOver true)
  (bind _asplayer_hud (Utilities|Casting|CastToPlayerHUD (HUD|GetHUD (Game|GetPlayerController 0)))))

(event EventBeginPlay
  (CallFunction|SpawnObjects)
  (Utilities|Time|SetTimerbyFunctionName 0 "SetGameStage" 1.5 true)
  (Audio|PlaySound2D "/Game/Sounds/Music/Timecrawler.Timecrawler" 1.0 1.0 0.0 0 0))

(fn ConstructionScript)

(fn SpawnObjects
  (bind _returnvalue (Math|Random|RandomUnitVector))
  (bind _max_generation_size (Variables|Default|GetMax%20Generation%20Size))
  (bind _objectdeviance (Variables|Default|GetObjectDeviance))
  (bind _returnvalue_2 (Math|Random|RandomFloatinRange 0.0 _max_generation_size))
  (bind _returnvalue_3 (* _objectdeviance -1.0))
  (bind _returnvalue_4 (* _returnvalue _returnvalue_2))
  (for _array_element (Variables|Default|GetSpawnableItems)
    (for _index (range 0 (Variables|Default|GetObjectsToGeneratePerType))
      (Game|SpawnActorfromClass _array_element (Math|Transform|MakeTransform (+ (Math|Vector|MakeVector (+ 0.0 (Math|Random|RandomFloatinRange _returnvalue_3 _objectdeviance)) 0.0 (Math|Float|Absolute(Float) (+ 0.0 (Math|Random|RandomFloatinRange _returnvalue_3 _objectdeviance)))) (Math|Vector|MakeVector (.x _returnvalue_4) 0.0 (Math|Float|Absolute(Float) (.z _returnvalue_4))))) "AdjustIfPossibleButDontSpawnIfColliding" 0 0))))