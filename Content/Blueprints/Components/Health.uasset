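; Health component that tracks damage and death for its owning actor.
; TakeDamage subtracts the amount, clamps Health at zero and passes the amount and killed state to OnTakeDamage.
; That event updates Alive and notifies the owner through IITakeDamageMessage, adding DeathMessage when killed.
; TakeDamage returns the killed flag, while its NewHealth output is always zero.
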(event Custom|OnTakeDamage
  (params (Amt :type Float%20%28single-precision%29) (Killed :type Boolean))
  (bind _returnvalue (Components|GetOwner))
  (Class|InteractionInterface|IITakeDamage(Message) _returnvalue)
  (bind _output_get (Variables|Default|SetAlive (not Killed)))
  (if (not _output_get)
    (Class|InteractionInterface|Death(Message) _returnvalue)))

(fn TakeDamage
  (params (Amt :type Float%20%28single-precision%29))
  (bind _output_get (Variables|Default|SetHealth (- (Variables|Default|GetHealth) Amt)))
  (if (<= _output_get 0.0)
    (Variables|Default|SetHealth 0.0))
  (CallFunction|OnTakeDamage Amt (<= _output_get 0.0))
  (return 0.0 (<= _output_get 0.0)))