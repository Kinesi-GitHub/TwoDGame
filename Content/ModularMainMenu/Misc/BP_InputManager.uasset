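; BP_InputManager is the input relay for the modular main menu, turning raw key presses into menu navigation commands.
; Hard-bound gamepad and keyboard key events (D-pad, arrows, WASD, face buttons, Space, Enter) converge into six actions: apply, back and four directions.
; Each action passes a string command to the referenced Widget's ButtonDispatcher, leaving all menu logic to that widget.
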(event Input|KeyboardEvents|SteamBackLeft
  (params (Key :type Key%20Structure))
  (:Pressed
    (Default|ButtonDispatcher (Variables|Default|GetWidget) "BACK")))

(event Input|KeyboardEvents|Up
  (params (Key :type Key%20Structure))
  (:Pressed
    (Default|ButtonDispatcher (Variables|Default|GetWidget) "UP")))

(event Input|KeyboardEvents|Down
  (params (Key :type Key%20Structure))
  (:Pressed
    (Default|ButtonDispatcher (Variables|Default|GetWidget) "DOWN")))

(event Input|GamepadEvents|GamepadFaceButtonRight
  (params (Key :type Key%20Structure))
  (:Pressed
    (Default|ButtonDispatcher (Variables|Default|GetWidget) "BACK")))

(event Input|KeyboardEvents|S
  (params (Key :type Key%20Structure))
  (:Pressed
    (Default|ButtonDispatcher (Variables|Default|GetWidget) "DOWN")))

(event Input|KeyboardEvents|W
  (params (Key :type Key%20Structure))
  (:Pressed
    (Default|ButtonDispatcher (Variables|Default|GetWidget) "UP")))

(event Input|KeyboardEvents|Enter
  (params (Key :type Key%20Structure))
  (:Pressed
    (Default|ButtonDispatcher (Variables|Default|GetWidget) "APPLY")))

(event Input|KeyboardEvents|SpaceBar
  (params (Key :type Key%20Structure))
  (:Pressed
    (Default|ButtonDispatcher (Variables|Default|GetWidget) "APPLY")))

(event Input|KeyboardEvents|A
  (params (Key :type Key%20Structure))
  (:Pressed
    (Default|ButtonDispatcher (Variables|Default|GetWidget) "LEFT")))

(event Input|KeyboardEvents|Left
  (params (Key :type Key%20Structure))
  (:Pressed
    (Default|ButtonDispatcher (Variables|Default|GetWidget) "LEFT")))

(event Input|GamepadEvents|GamepadDPadLeft
  (params (Key :type Key%20Structure))
  (:Pressed
    (Default|ButtonDispatcher (Variables|Default|GetWidget) "LEFT")))

(event Input|KeyboardEvents|D
  (params (Key :type Key%20Structure))
  (:Pressed
    (Default|ButtonDispatcher (Variables|Default|GetWidget) "RIGHT")))

(event Input|KeyboardEvents|Right
  (params (Key :type Key%20Structure))
  (:Pressed
    (Default|ButtonDispatcher (Variables|Default|GetWidget) "RIGHT")))

(event Input|GamepadEvents|GamepadDPadUp
  (params (Key :type Key%20Structure))
  (:Pressed
    (Default|ButtonDispatcher (Variables|Default|GetWidget) "UP")))

(event Input|GamepadEvents|GamepadDPadDown
  (params (Key :type Key%20Structure))
  (:Pressed
    (Default|ButtonDispatcher (Variables|Default|GetWidget) "DOWN")))

(event Input|GamepadEvents|GamepadFaceButtonBottom
  (params (Key :type Key%20Structure))
  (:Pressed
    (Default|ButtonDispatcher (Variables|Default|GetWidget) "APPLY")))

(event Input|GamepadEvents|GamepadDPadRight
  (params (Key :type Key%20Structure))
  (:Pressed
    (Default|ButtonDispatcher (Variables|Default|GetWidget) "RIGHT")))

(fn ConstructionScript)