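; Shared helper functions for the modular main menu system.
; Locates the level's single BP_ModularMainMenu actor, printing a long-lasting red error if none or several exist, and exposes its widget and macro lookup.
; A namespace filter merges the actor's global namespaces with the saved-namespace save game, keeping live values for the requested namespace and saved values for the rest.
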(fn FilterArraybyNamespace
  (params (namespace :type String))
  (SaveGame|CreateSaveGameObject "/Game/ModularMainMenu/Misc/BP_NamespaceSerialisation.BP_NamespaceSerialisation_C")
  (bind _returnvalue (SaveGame|LoadGamefromSlot "saved_namespace"))
  (bind _asbp_namespace_serialisation (Utilities|Casting|CastToBP_NamespaceSerialisation _returnvalue))
  (bind _outactors (Actor|GetAllActorsOfClass 0 "/Game/ModularMainMenu/Blueprints/BP_ModularMainMenu.BP_ModularMainMenu_C"))
  (for (_array_element _array_index) (Variables|/Game/ModularMainMenu/Blueprints/BP_ModularMainMenu.BP_ModularMainMenu_C|GetglobalNamespaces (Utilities|Array|Get(acopy) _outactors))
    (if (Utilities|Enum|Equal(Enum) namespace (.Namespace (Utilities|Struct|BreakSTR_Namespace _array_element)))
      (Utilities|Array|SetArrayElem (LocalVariables|GetlocalNamespaces) _array_index _array_element true)
      (else
        (Utilities|Array|SetArrayElem (LocalVariables|GetlocalNamespaces) _array_index (Utilities|Array|Get(acopy) (Variables|/Game/ModularMainMenu/Misc/BP_NamespaceSerialisation.BP_NamespaceSerialisation_C|GetNamespaceArray _asbp_namespace_serialisation) _array_index) true))))
  (return (LocalVariables|GetlocalNamespaces)))

(fn GetMenuWidget
  (bind _menubp (MenuGlobals|GetMenuBP))
  (return (Variables|/Game/ModularMainMenu/Blueprints/BP_ModularMainMenu.BP_ModularMainMenu_C|Getwidget _menubp)))

(fn GetMenuBP
  (bind _outactors (Actor|GetAllActorsOfClass 0 "/Game/ModularMainMenu/Blueprints/BP_ModularMainMenu.BP_ModularMainMenu_C"))
  (if (== (Utilities|Array|Length _outactors) 0)
    (MenuMisc|PrintMenuError "No ModularMainMenu_BP found on this map.")
    (elif (> (Utilities|Array|Length _outactors) 1)
      (MenuMisc|PrintMenuError "More than one ModularMainMenu_BP was  found on this map. You should use only one instance.")
      (else
        (return (Utilities|Array|Get(acopy) _outactors))))))

(fn PrintMenuError
  (params (Error :type String))
  (Development|PrintString 0 Error true true "(R=1.000000,G=0.000000,B=0.044828,A=1.000000)" 999.0))

(fn Macro
  (params (For :type String))
  (bind _menubp (MenuGlobals|GetMenuBP))
  (bind _result (Default|GetMacro _menubp For))
  (return _result))