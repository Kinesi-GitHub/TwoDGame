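; Helper functions for the modular main menu that store and persist string key-value settings grouped by namespace.
; Get and Set linearly search the GlobalNamespaces array on the first BP_ModularMainMenu actor.
; Typed "menu" accessors convert integers, floats, booleans and dash-joined 2D vectors to and from strings.
; Menu setters save the whole array to the "saved_namespace" slot, while SaveNamespace writes only one filtered namespace there.
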(fn GetGlobalVar
  (params (namespace :type String) (key :type String))
  (bind _outactors (Actor|GetAllActorsOfClass 0 "/Game/ModularMainMenu/Blueprints/BP_ModularMainMenu.BP_ModularMainMenu_C"))
  (bind _array_element (Utilities|Array|ForEachLoopwithBreak (Variables|/Game/ModularMainMenu/Blueprints/BP_ModularMainMenu.BP_ModularMainMenu_C|GetglobalNamespaces (Utilities|Array|Get(acopy) _outactors)) :!label _label)
    (:LoopBody
      (if (and (Utilities|Enum|Equal(Enum) (.Namespace (Utilities|Struct|BreakSTR_Namespace _array_element)) namespace) (Utilities|Enum|Equal(Enum) key (.Key (Utilities|Struct|BreakSTR_Namespace _array_element))))
        (LocalVariables|SetSavedValue (.Value (Utilities|Struct|BreakSTR_Namespace _array_element)))
        (Utilities|FlowControl|Sequence
          (:then_0
            (goto _label Break))
          (:then_1
            (return (LocalVariables|GetSavedValue) true)))))
    (:Completed
      (if (Utilities|Enum|Equal(Enum) (LocalVariables|GetSavedValue) "")
        (return "" false)))))

(fn SetGlobalVar
  (params (Namespace :type String) (Key :type String) (Value :type String))
  (bind _namespacestruct (Utilities|Struct|MakeSTR_Namespace Namespace Key Value))
  (bind _outactors (Actor|GetAllActorsOfClass 0 "/Game/ModularMainMenu/Blueprints/BP_ModularMainMenu.BP_ModularMainMenu_C"))
  (bind (_array_element _array_index) (Utilities|Array|ForEachLoopwithBreak (Variables|/Game/ModularMainMenu/Blueprints/BP_ModularMainMenu.BP_ModularMainMenu_C|GetglobalNamespaces (Utilities|Array|Get(acopy) _outactors)) :!label _label)
    (:LoopBody
      (if (and (Utilities|Enum|Equal(Enum) (.Namespace (Utilities|Struct|BreakSTR_Namespace _array_element)) Namespace) (Utilities|Enum|Equal(Enum) (.Key (Utilities|Struct|BreakSTR_Namespace _array_element)) Key))
        (Utilities|FlowControl|Sequence
          (:then_0
            (goto _label Break))
          (:then_1
            (Utilities|Array|SetArrayElem (Variables|/Game/ModularMainMenu/Blueprints/BP_ModularMainMenu.BP_ModularMainMenu_C|GetglobalNamespaces (Utilities|Array|Get(acopy) _outactors)) _array_index _namespacestruct true)
            (return)))))
    (:Completed
      (Utilities|Array|Add (Variables|/Game/ModularMainMenu/Blueprints/BP_ModularMainMenu.BP_ModularMainMenu_C|GetglobalNamespaces (Utilities|Array|Get(acopy) _outactors)) _namespacestruct)
      (return))))

(fn GetMenuString
  (params (key :type String))
  (bind _value (MenuSaves|GetGlobalVar "menu" key))
  (return _value))

(fn SetMenuString
  (params (Key :type String) (Value :type String))
  (MenuSaves|SetGlobalVar "menu" Key Value)
  (bind _returnvalue (SaveGame|CreateSaveGameObject "/Game/ModularMainMenu/Misc/BP_NamespaceSerialisation.BP_NamespaceSerialisation_C"))
  (bind _menubp (CallFunction|GetMenuBP))
  (Variables|/Game/ModularMainMenu/Misc/BP_NamespaceSerialisation.BP_NamespaceSerialisation_C|SetNamespaceArray _returnvalue (Variables|/Game/ModularMainMenu/Blueprints/BP_ModularMainMenu.BP_ModularMainMenu_C|GetglobalNamespaces _menubp))
  (SaveGame|SaveGametoSlot _returnvalue "saved_namespace"))

(fn SaveNamespace
  (params (namespace :type String))
  (bind _returnvalue (SaveGame|CreateSaveGameObject "/Game/ModularMainMenu/Misc/BP_NamespaceSerialisation.BP_NamespaceSerialisation_C"))
  (bind _out (CallFunction|FilterArraybyNamespace namespace))
  (Variables|/Game/ModularMainMenu/Misc/BP_NamespaceSerialisation.BP_NamespaceSerialisation_C|SetNamespaceArray _returnvalue _out)
  (SaveGame|SaveGametoSlot _returnvalue "saved_namespace"))

(fn GetMenuInteger
  (params (key :type String))
  (bind _value (MenuSaves|GetMenuString key))
  (return (Math|Conversions|ToInteger(Byte) _value)))

(fn GetMenuFloat
  (params (key :type String))
  (bind _value (MenuSaves|GetMenuString key))
  (return (Math|Conversions|ToFloat(Integer) _value)))

(fn GetMenuBoolean
  (params (key :type String))
  (bind _value (MenuSaves|GetMenuString key))
  (return (Utilities|Enum|Equal(Enum) _value "true")))

(fn GetMenuVector
  (params (key :type String))
  (bind _value (MenuSaves|GetMenuString key))
  (return (Math|Vector2D|MakeVector2D (Math|Conversions|ToFloat(Integer) (.LeftS (Utilities|String|Split _value "-"))) (Math|Conversions|ToFloat(Integer) (.RightS (Utilities|String|Split _value "-"))))))

(fn SetMenuInteger
  (params (key :type String) (Integer :type Integer))
  (MenuSaves|SetMenuString key (Utilities|String|ToString(Integer) Integer))
  (return))

(fn SetMenuFloat
  (params (key :type String) (value :type Float%20%28single-precision%29))
  (MenuSaves|SetMenuString key (Utilities|String|ToString(Float) value))
  (return))

(fn SetMenuBoolean
  (params (key :type String) (value :type Boolean))
  (MenuSaves|SetMenuString key (select value "true" "false"))
  (return))

(fn SetMenuVector
  (params (key :type String) (value :type Vector%202D%20Structure))
  (bind (_x _y) (Math|Vector2D|BreakVector2D value))
  (MenuSaves|SetMenuString key (Utilities|String|Append (Utilities|String|ToString(Float) _x) "-" (Utilities|String|ToString(Float) _y)))
  (return))