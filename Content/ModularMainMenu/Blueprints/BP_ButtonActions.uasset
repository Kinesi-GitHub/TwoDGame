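; Button action handler for the modular main menu, mapping action IDs from the menu data table to game behavior.
; CustomAction dispatches quit, continue (closes the in-game menu), and graphics or video updates; New Game only prints a setup error.
; The update functions read saved menu values by key and apply them as console commands.
; The field-of-view setting is an unconnected placeholder awaiting a camera.
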(fn CustomAction
  (params (action :type String))
  (switch string action ; Add your custom action for buttons here. Action string ID should match the ID you defined in the data table.
    (:ExitGame
      (MenuDefaultActions|CloseGame))
    (:ContinueGame
      (MenuDefaultActions|Continue))
    (:UpdateGraphics
      (|UpdateGraphics))
    (:UpdateVideo
      (|UpdateVideo))
    (:NewGame
      (CallFunction|PrintMenuError "No action assigned for the New Game button. Assign an action in the \"ModularMainMenu/Blueprints/ButtonActions\" blueprint or enter a level name in the data table. "))))

(fn Continue
  (bind _menubp (CallFunction|GetMenuBP))
  (if (Variables|/Game/ModularMainMenu/Blueprints/BP_ModularMainMenu.BP_ModularMainMenu_C|GetisInGame _menubp)
    (Default|CloseMenu _menubp)))

(fn CloseGame
  (Game|QuitGame 0 0 "Quit" false))